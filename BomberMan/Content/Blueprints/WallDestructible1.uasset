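; Destructible wall Blueprint that can drop a random power-up at its cube's location.
; PickUpChance tests in turn for a bomb-count, blast-range or speed pickup, spawning at most one.
; Each comparison makes its own random roll, so the odds cascade and the speed check is not a single narrow band.
; The event graph and construction script are empty, and nothing here calls PickUpChance or handles destruction.
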(fn `PickUpChance`
  (bind _returnvalue (`KismetMathLibrary.RandomFloatInRange` 0.0 10.0))
  (bind _returnvalue_2 (`SceneComponent.K2_GetComponentLocation` (`self.Cube`)))
  ;[1 1 1] Drop the pickup that increase the max amount of bomb can be active a time if random number < 1
  (if (< _returnvalue 1.0)
    (`|SpawnActorFromClass` "/Game/Blueprints/PickUpBombAmountIncrease.PickUpBombAmountIncrease_C" (`KismetMathLibrary.Conv_VectorToTransform` _returnvalue_2) "Undefined" "OverrideRootScale" null null)
    (else
      ;[1 1 1] Drop the pickup that increase the bomb blast range if random number > 9
      (if (> _returnvalue 9.0)
        (`|SpawnActorFromClass` "/Game/Blueprints/PickUpBombRangeIncrease.PickUpBombRangeIncrease_C" (`KismetMathLibrary.Conv_VectorToTransform` _returnvalue_2) "Undefined" "OverrideRootScale" null null)
        (else
          ;[1 1 1] Drop the pickup that increase the speed of player if 4.5 < random number < 5.5
          (if (and (< _returnvalue 5.5) (> _returnvalue 4.5))
            (`|SpawnActorFromClass` "/Game/Blueprints/PickUpSpeedIncrease.PickUpSpeedIncrease_C" (`KismetMathLibrary.Conv_VectorToTransform` _returnvalue_2) "Undefined" "OverrideRootScale" null null)))))))

(fn `UserConstructionScript`)