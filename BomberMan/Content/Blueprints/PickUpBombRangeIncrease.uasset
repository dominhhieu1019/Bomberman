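; Bomb range pickup that extends a player's bomb blast range when touched.
; On sphere overlap it checks whether the actor's class is Player1 or Player2 and adds a fixed amount to that player's range variable in NewGameInstance.
; The pickup then destroys itself, and other overlapping actors leave it untouched.
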(event `self.Sphere1.OnComponentBeginOverlap`
  (params (OverlappedComponent :type "PrimitiveComponent Object Reference") (OtherActor :type "Actor Object Reference") (OtherComp :type "PrimitiveComponent Object Reference") (OtherBodyIndex :type Integer) (bFromSweep :type Boolean) (SweepResult :type "HitResult Structure (by ref)"))
  (bind _returnvalue (`GameplayStatics.GetObjectClass` OtherActor))
  (bind _returnvalue_2 (`GameplayStatics.GetGameInstance`))
  ;[1 1 1] Player 1 increase the bomb blast range
  (if (== _returnvalue "/Game/Blueprints/Player1.Player1_C")
    (bind _asnew_game_instance (cast `/Game/Blueprints/NewGameInstance` _returnvalue_2))
    (set `/Game/Blueprints/NewGameInstance.P1BombRange` (+ (`/Game/Blueprints/NewGameInstance.P1BombRange` _asnew_game_instance) 40.0) _asnew_game_instance)
    (`self.K2_DestroyActor` :!label _label)
    (else
      ;[1 1 1] Player 2 increase the bomb blast range
      (if (== _returnvalue "/Game/Blueprints/Player2.Player2_C")
        (bind _asnew_game_instance_2 (cast `/Game/Blueprints/NewGameInstance` _returnvalue_2))
        (set `/Game/Blueprints/NewGameInstance.P2BombRange` (+ (`/Game/Blueprints/NewGameInstance.P2BombRange` _asnew_game_instance_2) 40.0) _asnew_game_instance_2)
        (goto _label)))))

(fn `UserConstructionScript`)