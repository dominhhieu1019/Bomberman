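; Player 2's controllable character, which moves around and drops bombs.
; Each tick it pushes its Cube with a physics force from the Up2/Right2 input, or resets bomb and speed stats while the game instance's EndGame flag is set.
; Slash spawns a Bomb1_Player2 above the cube and increments the placed count, gated by Bombs <= MaxBombs, which allows one more than MaxBombs.
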(event `self.ReceiveBeginPlay`
  (bind _asnew_game_instance (cast `/Game/Blueprints/NewGameInstance` (`GameplayStatics.GetGameInstance`)))
  (set `self.gameInstance` _asnew_game_instance))

(event `self.ReceiveTick`
  (params (DeltaSeconds :type "Float (single-precision)"))
  ;[1 1 1] Movement
  (`self.Movement`))

(event `Key|Slash`
  (params (Key :type "Key Structure"))
  ;[1 1 1] Spawm Bomb
  (:`Pressed`
    (`self.PlaceBomb`)))

(fn `Movement`
  (bind _runspeed (`self.runSpeed`))
  (if (`/Game/Blueprints/NewGameInstance.EndGame` (`self.gameInstance`))
    ;[1 1 1] Set max bomb, placed bomb and speed to default values
    (set `self.maxBombs` 1)
    (set `self.bombs` 0)
    (set `self.runSpeed` 300000)
    (else
      ;[1 1 1] Get direction
      (`PrimitiveComponent.AddForce` (`self.Cube`) (`KismetMathLibrary.MakeVector` (* (`self.GetInputAxisValue`) (`KismetMathLibrary.Conv_IntToDouble` _runspeed)) (* (`self.GetInputAxisValue`) (`KismetMathLibrary.Conv_IntToDouble` _runspeed))) "None" false))))

(fn `PlaceBomb`
  ;[1 1 1] Check if placed bombs < max bombs
  (if (<= (`self.bombs`) (`self.maxBombs`))
    (`|SpawnActorFromClass` "/Game/Blueprints/Bomb1_Player2.Bomb1_Player2_C" (`KismetMathLibrary.Conv_VectorToTransform` (`KismetMathLibrary.MakeVector` (.x (`SceneComponent.K2_GetComponentLocation` (`self.Cube`))) (.y (`SceneComponent.K2_GetComponentLocation` (`self.Cube`))) (+ (.z (`SceneComponent.K2_GetComponentLocation` (`self.Cube`))) 150.0))) "Undefined" "OverrideRootScale" null null)
    (`/Engine/EditorBlueprintResources/StandardMacros.IncrementInt` (`self.bombs`))))

(fn `UserConstructionScript`)