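; Player 2's bomb actor, which explodes after a short fuse and destroys what is in its blast radius.
; On BeginPlay it sizes a sphere from the GameInstance's P2BombRange, waits, then decrements Bombs on every Player2 actor.
; Sphere overlaps are filtered by class: destructible walls roll a pickup chance, players set their death flag on the GameInstance, and these plus pickups are destroyed.
; The bomb then destroys itself.
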(event `self.ReceiveBeginPlay`
  (bind _returnvalue (`GameplayStatics.GetGameInstance`))
  ;[1 1 1] Set bome blast range
  (bind _asnew_game_instance (cast `/Game/Blueprints/NewGameInstance` (`GameplayStatics.GetGameInstance`)))
  (set `self.gameInstance` _asnew_game_instance)
  (`SphereComponent.SetSphereRadius` (`self.Sphere1`) (`/Game/Blueprints/NewGameInstance.P2BombRange` (`self.gameInstance`)) true)
  (`KismetSystemLibrary.Delay` 2.0) ; Time before bomb explodes
  (bind _outactors (`GameplayStatics.GetAllActorsOfClass` "/Game/Blueprints/Player2.Player2_C"))
  (for _array_element _outactors
    ;[1 1 1] Increase the amount of bombs player can place when the bomb placed before explodes
    (`/Engine/EditorBlueprintResources/StandardMacros.DecrementInt` (`/Game/Blueprints/Player2.bombs` _array_element)))
  ;[1 1 1] Get set of players or pickups in bomb blast range
  (bind _output_get (set `self.overlapping` (`PrimitiveComponent.GetOverlappingActors` (`self.Sphere1`) null)))
  (for _array_element_2 _output_get
    (bind _returnvalue_2 (`GameplayStatics.GetObjectClass` _array_element_2))
    ;[1 1 1] Break destructible wall and drop pickups if any
    (if (== _returnvalue_2 "/Game/Blueprints/WallDestructible1.WallDestructible1_C")
      (bind _aswall_destructible_1 (cast `/Game/Blueprints/WallDestructible1` _array_element_2))
      (`/Game/Blueprints/WallDestructible1.PickUpChance` _aswall_destructible_1)
      (`self.K2_DestroyActor` _array_element_2 :!label _label)
      (else
        ;[1 1 1] Destroy player if standing in bomb blast range and set 'alive' variable of the died player to 'false'
        (if (== _returnvalue_2 "/Game/Blueprints/Player1.Player1_C")
          (bind _asnew_game_instance_2 (cast `/Game/Blueprints/NewGameInstance` _returnvalue)
            (:`then`
              _)
            (:`CastFailed`
              _))
          (set `/Game/Blueprints/NewGameInstance.P1Death` true _asnew_game_instance_2)
          (goto _label)
          (elif (== _returnvalue_2 "/Game/Blueprints/Player2.Player2_C")
            (bind _asnew_game_instance_3 (cast `/Game/Blueprints/NewGameInstance` _returnvalue)
              (:`then`
                _)
              (:`CastFailed`
                _))
            (set `/Game/Blueprints/NewGameInstance.P2Death` true _asnew_game_instance_3)
            (goto _label)
            (else
              ;[1 1 1] Destroy pickups if they are in bomb blash range
              (if (== _returnvalue_2 "/Game/Blueprints/PickUpBombAmountIncrease.PickUpBombAmountIncrease_C")
                (goto _label)
                (elif (== null _returnvalue_2)
                  (goto _label)
                  (elif (== null _returnvalue_2)
                    (goto _label))))))))))
  (`self.K2_DestroyActor`))

(fn `UserConstructionScript`)