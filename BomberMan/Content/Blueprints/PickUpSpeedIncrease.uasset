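; PickUpSpeedIncrease is a pickup that boosts the run speed of Player1 or Player2 on contact.
; An overlap on Sphere1 checks the other actor's exact class, casts it and adds a large fixed amount to its RunSpeed variable.
; Both player branches then destroy the pickup, and nothing in this Blueprint reverts the boost.
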(event `self.Sphere1.OnComponentBeginOverlap`
  (params (OverlappedComponent :type "PrimitiveComponent Object Reference") (OtherActor :type "Actor Object Reference") (OtherComp :type "PrimitiveComponent Object Reference") (OtherBodyIndex :type Integer) (bFromSweep :type Boolean) (SweepResult :type "HitResult Structure (by ref)"))
  (bind _returnvalue (`GameplayStatics.GetObjectClass` OtherActor))
  ;[1 1 1] Player 1 pick up Speed booster
  (if (== _returnvalue "/Game/Blueprints/Player1.Player1_C")
    (bind _asplayer_1 (cast `/Game/Blueprints/Player1` OtherActor))
    (set `/Game/Blueprints/Player1.runSpeed` (+ (`/Game/Blueprints/Player1.runSpeed` _asplayer_1) 100000) _asplayer_1)
    (`self.K2_DestroyActor` :!label _label)
    (else
      ;[1 1 1] Player 2 pick up Speed booster
      (if (== _returnvalue "/Game/Blueprints/Player2.Player2_C")
        (bind _asplayer_2 (cast `/Game/Blueprints/Player2` OtherActor))
        (set `/Game/Blueprints/Player2.runSpeed` (+ (`/Game/Blueprints/Player2.runSpeed` _asplayer_2) 100000) _asplayer_2)
        (goto _label)))))

(fn `UserConstructionScript`)